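; ComfortZone is a placeable area that gradually lowers the player's Fear while they stand inside it.
; Box overlap begin and end events, filtered to FPSController, toggle a PlayerInZone flag.
; While the flag is set, Tick finds the FPSController via GetActorOfClass and subtracts DeFearValue scaled by delta time whenever Fear is above zero, without clamping the result.
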(event OnComponentBeginOverlap(Box)
  (params (OverlappedComponent :type Primitive%20Component%20Object%20Reference) (OtherActor :type Actor%20Object%20Reference) (OtherComp :type Primitive%20Component%20Object%20Reference) (OtherBodyIndex :type Integer) (bFromSweep :type Boolean) (SweepResult :type Hit%20Result%20Structure%20%28by%20ref%29))
  (Utilities|Casting|CastToFPSController OtherActor)
  (Variables|Default|SetPlayerInZone true))

(event OnComponentEndOverlap(Box)
  (params (OverlappedComponent :type Primitive%20Component%20Object%20Reference) (OtherActor :type Actor%20Object%20Reference) (OtherComp :type Primitive%20Component%20Object%20Reference) (OtherBodyIndex :type Integer))
  (Utilities|Casting|CastToFPSController OtherActor)
  (Variables|Default|SetPlayerInZone false))

(event EventBeginPlay)

(event Collision|EventActorBeginOverlap
  (params (OtherActor :type Actor%20Object%20Reference)))

(event EventTick
  (params (DeltaSeconds :type Float%20%28single-precision%29))
  (if (Variables|Default|GetPlayerInZone)
    (bind _returnvalue (Actor|GetActorOfClass "/Game/Blueprints/FPSController.FPSController_C"))
    (if (> (Variables|/Game/Blueprints/FPSController.FPSController_C|GetFear _returnvalue) 0.0)
      (bind _output_get (Variables|/Game/Blueprints/FPSController.FPSController_C|SetFear _returnvalue (- (stale _output_get) (* (Variables|Default|GetDe-FearValue) DeltaSeconds)))))))

(fn ConstructionScript)