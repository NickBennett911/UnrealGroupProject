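; Volume actor that periodically makes the SpookyGhost appear at a random floor spot inside its bounds and wander briefly before being sent home.
; Tick runs a random spawn countdown, then traces for a Floor-tagged component, moves the ghost there and plays a sound.
; Radial line traces turn the ghost toward the first unobstructed or farthest-hit direction.
; Wander time shrinks as the player's PlacesVisited count grows.
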(event EventBeginPlay
  (CallFunction|SetTimer)
  (bind _returnvalue (Actor|GetActorOfClass "/Game/Blueprints/SpookyGhost.SpookyGhost_C"))
  (Variables|Default|SetGhostRef _returnvalue)
  (bind _returnvalue_2 (Actor|GetActorOfClass "/Game/Blueprints/FPSController.FPSController_C"))
  (Variables|Default|SetPlayerRef _returnvalue_2))

(event EventTick
  (params (DeltaSeconds :type Float%20%28single-precision%29))
  (bind _ghostwandervolume (Variables|Default|GetGhostWanderVolume))
  (bind _ghostref (Variables|Default|GetGhostRef))
  (bind _ghostref_2 (Variables|Default|GetGhostRef))
  (bind _returnvalue (Transformation|GetWorldLocation _ghostwandervolume))
  (bind _returnvalue_2 (Components|Box|GetScaledBoxExtent _ghostwandervolume))
  (bind _returnvalue_3 (Math|Random|RandomPointinBoundingBox _returnvalue _returnvalue_2))
  (if (Variables|/Game/Blueprints/SpookyGhost.SpookyGhost_C|GetIsWandering (Variables|Default|GetGhostRef))
    ;[1 1 1] while ghost is wandering
    (bind _output_get (Variables|Default|SetWanderTimer (- (stale _output_get) DeltaSeconds)))
    ;;[1 1 1] if ghost is done wander then send him to his home location and stop wandering
    (if (< (Variables|Default|GetWanderTimer) 0.0)
      (Default|SendHome _ghostref)
      (Variables|/Game/Blueprints/SpookyGhost.SpookyGhost_C|SetIsWandering _ghostref false)
      (Audio|Components|Audio|Stop (Variables|/Game/Blueprints/SpookyGhost.SpookyGhost_C|GetGhostWanderSound _ghostref)))
    (else
      (bind _output_get_2 (Variables|Default|SetSpawnTimer (- (stale _output_get_2) DeltaSeconds)))
      (if (< (Variables|Default|GetSpawnTimer) 0.0)
        (CallFunction|SetTimer)
        (bind (_outhit _returnvalue_4) (Collision|LineTraceByChannel _returnvalue_3 (+ _returnvalue_3 (* (Math|Vector|MakeVector 0.0 0.0 -1.0) (Variables|Default|GetDownwardLineTraceDist))) "TraceTypeQuery1" false 0 "None"))
        (if _returnvalue_4
          (if (Components|ComponentHasTag (.HitComponent (Collision|BreakHitResult _outhit)) "Floor")
            (Transformation|SetWorldLocation (Variables|/Game/Blueprints/SpookyGhost.SpookyGhost_C|GetGhost _ghostref_2) (.Location (Collision|BreakHitResult _outhit)) false false)
            (Audio|PlaySoundatLocation "/Game/Sounds/Wav/WanderGhostSpawnSound.WanderGhostSpawnSound" (.Location (Collision|BreakHitResult _outhit)) "0, 0, 0" 1.0 1.0 0.0 0 0 0)
            (bind _direction (CallFunction|FindGhostLookDirection (.Location (Collision|BreakHitResult _outhit)) 8.0))
            (CallFunction|GhostLookat _direction)
            (Variables|/Game/Blueprints/SpookyGhost.SpookyGhost_C|SetIsWandering _ghostref_2 true)))))))

(fn ConstructionScript)

(fn SetTimer
  (Variables|Default|SetSpawnTimer (Math|Random|RandomFloatinRange 3e+01 45.0))
  (bind _returnvalue (Actor|GetActorOfClass "/Game/Blueprints/FPSController.FPSController_C"))
  (Variables|Default|SetWanderTimer (/ 6.0 (Math|Conversions|ToFloat(Integer) (+ (Variables|/Game/Blueprints/FPSController.FPSController_C|GetPlacesVisited _returnvalue) 1)))))

(fn FindGhostLookDirection
  (params (SpawnLocation :type Vector) (Precision :type Float%20%28single-precision%29))
  (LocalVariables|SetGhostLocation SpawnLocation)
  (LocalVariables|SetAngleStep (/ 3.6e+02 Precision))
  (bind _index (Utilities|FlowControl|ForLoopwithBreak 0 (- (Math|Float|Truncate Precision) 1))
    (:LoopBody
      (bind _resultingvector (CallFunction|MakeVectorfromAngle (* _index (LocalVariables|GetAngleStep))))
      (LocalVariables|SetTempDir _resultingvector)
      (bind (_outhit _returnvalue) (Collision|LineTraceByChannel (+ (LocalVariables|GetGhostLocation) (LocalVariables|GetGhostVertOffset)) (+ (+ (LocalVariables|GetGhostLocation) (LocalVariables|GetGhostVertOffset)) (* _resultingvector (LocalVariables|GetLineTraceDist))) "TraceTypeQuery1" false 0 "None"))
      (if _returnvalue
        (if (> (.Distance (Collision|BreakHitResult _outhit)) (LocalVariables|GetRecordDist))
          (LocalVariables|SetRecordDist (.Distance (Collision|BreakHitResult _outhit)))
          (LocalVariables|SetRecordDir (LocalVariables|GetTempDir)))
        (else
          ;[1 1 1] If no hit then ghost has plenty of room to go that direction, no reason to look at other locations
          (return (LocalVariables|GetTempDir)))))
    (:Completed
      (return (LocalVariables|GetRecordDir)))))

(fn MakeVectorfromAngle
  (params (Angle :type Float%20%28single-precision%29))
  (return (Math|Vector|RotateVector (LocalVariables|GetDirection) (Math|Vector|RotatorfromAxisandAngle (Math|Vector|GetUpVector (Variables|/Game/Blueprints/SpookyGhost.SpookyGhost_C|GetGhost (Variables|Default|GetGhostRef))) Angle))))

(fn GhostLookat
  (params (Direction :type Vector))
  (Transformation|SetActorRotation (Variables|Default|GetGhostRef) (Math|Rotator|MakeRotator 0.0 0.0 (- (.yaw (Math|Conversions|RotationFromXVector Direction)) 9e+01))))