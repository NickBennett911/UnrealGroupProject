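; SoundEventParent is a ghost event trigger, named as a parent class, that plays a random sound when the player walks into it.
; When an FPSController overlaps the Collider, it plays one of three audio components, picked by weighted thresholds on a float rolled at BeginPlay.
; A HasPlayedSound flag makes it one-shot; the float is re-rolled afterwards, though nothing here resets the flag.
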(event OnComponentBeginOverlap(Collider)
  (params (OverlappedComponent :type Primitive%20Component%20Object%20Reference) (OtherActor :type Actor%20Object%20Reference) (OtherComp :type Primitive%20Component%20Object%20Reference) (OtherBodyIndex :type Integer) (bFromSweep :type Boolean) (SweepResult :type Hit%20Result%20Structure%20%28by%20ref%29))
  (if (not (Variables|Default|GetHasPlayedSound))
    (Utilities|Casting|CastToFPSController OtherActor)
    (if (< (Variables|Default|GetRandom) 0.3)
      (Audio|Components|Audio|Play (Variables|Default|GetNoise) 0.0)
      (Variables|Default|SetHasPlayedSound true)
      (Variables|Default|SetRandom (Math|Random|RandomFloat) :!label _label)
      (elif (< (Variables|Default|GetRandom) 0.7)
        (Audio|Components|Audio|Play (Variables|Default|GetAudio_2) 0.0)
        (Variables|Default|SetHasPlayedSound true)
        (goto _label)
        (elif (< (Variables|Default|GetRandom) 1.1)
          (Audio|Components|Audio|Play (Variables|Default|GetAudio_3) 0.0)
          (Variables|Default|SetHasPlayedSound true)
          (goto _label))))))

(event EventBeginPlay
  (Variables|Default|SetRandom (Math|Random|RandomFloat)))

(event Collision|EventActorBeginOverlap
  (params (OtherActor :type Actor%20Object%20Reference)))

(event EventTick
  (params (DeltaSeconds :type Float%20%28single-precision%29)))

(fn ConstructionScript)