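; Ghost scare event that, on first player overlap with its collider, places a ghost mesh behind the player and plays a spawn sound.
; Tick turns the ghost toward the player and advances it, adding FPSController Fear while a camera dot-product test finds it near view center.
; It returns home when its timer expires or it gets close enough.
; SetEventSeverity supplies tuning presets, with the lowest applied on BeginPlay.
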(event OnComponentBeginOverlap(Collider)
  (params (OverlappedComponent :type Primitive%20Component%20Object%20Reference) (OtherActor :type Actor%20Object%20Reference) (OtherComp :type Primitive%20Component%20Object%20Reference) (OtherBodyIndex :type Integer) (bFromSweep :type Boolean) (SweepResult :type Hit%20Result%20Structure%20%28by%20ref%29))
  (Utilities|Casting|CastToFPSController OtherActor)
  (if (not (Variables|Default|GetSeekPlayer))
    (bind _mesh (CallFunction|GetPlayerMesh))
    (Transformation|SetWorldLocation (Variables|Default|GetSkeletalMesh) (+ (* (Math|Vector|MakeVector (* (.x (Math|Vector|GetForwardVector _mesh)) -1.0) (* (.y (Math|Vector|GetForwardVector _mesh)) -1.0) 0.0) (Variables|Default|GetGhostToPlayerSpawnDist)) (Transformation|GetWorldLocation _mesh)) false false)
    (Transformation|SetWorldRotation (Variables|Default|GetSkeletalMesh) (Math|Rotator|MakeRotator 0.0 0.0 (- (.yaw (Math|Rotator|FindLookatRotation (Transformation|GetWorldLocation (Variables|Default|GetSkeletalMesh)) (Transformation|GetWorldLocation _mesh))) 9e+01)) false false)
    (Variables|Default|SetSeekPlayer true)
    (Variables|Default|SetHandleGhost true)
    (Audio|Components|Audio|Play (Variables|Default|GetGhostSpawnSound) (Variables|Default|GetSoundStartTime))))

(event EventBeginPlay
  (CallFunction|SetEventSeverity))

(event EventTick
  (params (DeltaSeconds :type Float%20%28single-precision%29))
  (bind _skeletalmesh (Variables|Default|GetSkeletalMesh))
  (if (Variables|Default|GetHandleGhost)
    (bind _shoulddespawnghost (CallFunction|DespawnGhost DeltaSeconds))
    (if _shoulddespawnghost
      (Transformation|SetWorldLocation (Variables|Default|GetSkeletalMesh) (Variables|Default|GetGhostHomeLocation) false false)
      (Variables|Default|SetHandleGhost false)
      (elif (Variables|Default|GetSeekPlayer)
        (bind _mesh (CallFunction|GetPlayerMesh))
        (Transformation|SetWorldRotation _skeletalmesh (Math|Rotator|MakeRotator 0.0 0.0 (- (.yaw (Math|Rotator|FindLookatRotation (Transformation|GetWorldLocation (Variables|Default|GetSkeletalMesh)) (Transformation|GetWorldLocation _mesh))) 9e+01)) false false)
        (Transformation|AddActorLocalOffset (* (Math|Vector|GetRightVector _skeletalmesh) (* DeltaSeconds (Variables|Default|GetGhostSpeed))) false false)
        (CallFunction|InFrame)))))

(fn ConstructionScript)

(fn GetPlayerMesh
  (bind _returnvalue (Actor|GetActorOfClass "/Game/Blueprints/FPSController.FPSController_C"))
  (return (Variables|/Script/Engine.Character|GetMesh _returnvalue)))

(fn DespawnGhost
  (params (deltaTime :type Float%20%28single-precision%29))
  (bind _output_get (Variables|Default|SetDespawnTimer (- (stale _output_get) deltaTime)))
  (if (< _output_get 0.0)
    (return true)
    (else
      (bind _returnvalue (Actor|GetActorOfClass "/Game/Blueprints/FPSController.FPSController_C"))
      (return (<= (Math|Vector|VectorLength (- (Transformation|GetWorldLocation (Variables|/Script/Engine.Character|GetMesh _returnvalue)) (Transformation|GetWorldLocation (Variables|Default|GetSkeletalMesh)))) (Variables|Default|GetDespawnGhostDist))))))

(fn InFrame
  (bind _returnvalue (Actor|GetActorOfClass "/Game/Blueprints/FPSController.FPSController_C"))
  (bind _output_get (Variables|Default|SetVectorToObject (Math|Vector|Normalize (- (Transformation|GetWorldLocation (Variables|Default|GetSkeletalMesh)) (Transformation|GetWorldLocation (Variables|/Script/Engine.Character|GetMesh _returnvalue))))))
  (if (> (Math|Vector|DotProduct _output_get (Math|Vector|GetForwardVector (Variables|/Game/Blueprints/FPSController.FPSController_C|GetCamera _returnvalue))) 0.95)
    (CallFunction|AddFear (Variables|Default|GetFearAmnt))))

(fn AddFear
  (params (Amnt :type Float%20%28single-precision%29))
  (bind _returnvalue (Actor|GetActorOfClass "/Game/Blueprints/FPSController.FPSController_C"))
  (bind _output_get (Variables|/Game/Blueprints/FPSController.FPSController_C|SetFear _returnvalue (+ (stale _output_get) Amnt))))

(fn SetEventSeverity
  (params (Severity :type Integer))
  (if (== Severity 0)
    (Variables|Default|SetGhostSpeed 1.5e+02)
    (Variables|Default|SetDespawnGhostDist 8e+02)
    (Variables|Default|SetGhostToPlayerSpawnDist 1000)
    (Variables|Default|SetDespawnTimer 4.0)
    (elif (== Severity 1)
      (Variables|Default|SetGhostSpeed 275.0)
      (Variables|Default|SetDespawnGhostDist 5e+02)
      (Variables|Default|SetGhostToPlayerSpawnDist 700)
      (Variables|Default|SetDespawnTimer 4.0)
      (Variables|Default|SetSoundStartTime 1.5)
      (Variables|Default|SetFearAmnt 0.1)
      (elif (== Severity 2)
        (Variables|Default|SetGhostSpeed 3e+02)
        (Variables|Default|SetDespawnGhostDist 3e+02)
        (Variables|Default|SetGhostToPlayerSpawnDist 600)
        (Variables|Default|SetDespawnTimer 4.0)
        (Variables|Default|SetSoundStartTime 1.5)
        (Variables|Default|SetFearAmnt 0.15)
        (elif (== Severity 3)
          (Variables|Default|SetGhostSpeed 475.0)
          (Variables|Default|SetDespawnGhostDist 0.0)
          (Variables|Default|SetGhostToPlayerSpawnDist 400)
          (Variables|Default|SetDespawnTimer 3.0)
          (Variables|Default|SetSoundStartTime 1.5)
          (Variables|Default|SetFearAmnt 0.2)
          (else
            (Development|PrintString "Invalid severity level given in set event severity in spwn behind event")))))))