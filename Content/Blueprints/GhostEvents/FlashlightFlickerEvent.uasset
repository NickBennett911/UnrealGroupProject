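; One-shot trigger box scare that flickers the player's flashlight and spawns the SpookyGhost ahead of them.
; SeverityLevel (0-3) selects flicker timing, ghost speed, spawn sound and fear added to the FPSController.
; After the spawn animation, Tick adds fear each frame the ghost is within the camera's forward cone (dot product test).
; When the despawn timer expires, the ghost mesh drops far below the world and stops tracking.
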(event OnComponentBeginOverlap(Box)
  (params (OverlappedComponent :type Primitive%20Component%20Object%20Reference) (OtherActor :type Actor%20Object%20Reference) (OtherComp :type Primitive%20Component%20Object%20Reference) (OtherBodyIndex :type Integer) (bFromSweep :type Boolean) (SweepResult :type Hit%20Result%20Structure%20%28by%20ref%29))
  (if (not (Variables|Default|GetEventUsed))
    (bind _asfpscontroller (Utilities|Casting|CastToFPSController OtherActor))
    (if (== (Variables|Default|GetSeverityLevel) 0)
      (bind _ghostref (CallFunction|SetSeverityZero _asfpscontroller))
      (bind _ghostrefout (CallFunction|SetGhostLocation _ghostref _asfpscontroller))
      (Variables|/Game/Blueprints/SpookyGhost.SpookyGhost_C|SetTrackPlayer _ghostrefout true)
      (Audio|Components|Audio|Play (Variables|/Game/Blueprints/SpookyGhost.SpookyGhost_C|GetGhostSpawnSound _ghostrefout) 1.2)
      (CallFunction|AddFear 2.0)
      (elif (== (Variables|Default|GetSeverityLevel) 1)
        (bind _ghostref_2 (CallFunction|SetSeverityOne _asfpscontroller))
        (bind _ghostrefout_2 (CallFunction|SetGhostLocation _ghostref_2 _asfpscontroller))
        (Variables|/Game/Blueprints/SpookyGhost.SpookyGhost_C|SetTrackPlayer _ghostrefout_2 true)
        (Audio|Components|Audio|Play (Variables|/Game/Blueprints/SpookyGhost.SpookyGhost_C|GetGhostSpawnSound _ghostrefout_2) 1.0)
        (CallFunction|AddFear 3.5)
        (Variables|Default|SetFearAmount 0.08)
        (elif (== (Variables|Default|GetSeverityLevel) 2)
          (bind _ghostref_3 (CallFunction|SetSeverityTwo _asfpscontroller))
          (bind _ghostrefout_3 (CallFunction|SetGhostLocation _ghostref_3 _asfpscontroller))
          (Variables|/Game/Blueprints/SpookyGhost.SpookyGhost_C|SetTrackPlayer _ghostrefout_3 true)
          (Audio|Components|Audio|Play (Variables|/Game/Blueprints/SpookyGhost.SpookyGhost_C|GetGhostSpawnSound _ghostrefout_3) 1.0)
          (CallFunction|AddFear 5.5)
          (Variables|Default|SetFearAmount 0.1)
          (elif (== (Variables|Default|GetSeverityLevel) 3)
            (bind _ghostref_4 (CallFunction|SetSeverityThree _asfpscontroller))
            (bind _ghostrefout_4 (CallFunction|SetGhostLocation _ghostref_4 _asfpscontroller))
            (Variables|/Game/Blueprints/SpookyGhost.SpookyGhost_C|SetTrackPlayer _ghostrefout_4 true)
            (Audio|Components|Audio|Play (Variables|/Game/Blueprints/SpookyGhost.SpookyGhost_C|GetGhostSpawnSound _ghostrefout_4) 1.5)
            (CallFunction|AddFear 8.0)
            (Variables|Default|SetFearAmount 0.5)
            (else
              (Development|PrintString "Invalid Severity Level Given To Flicker Event"))))))))

(event EventBeginPlay)

(event Collision|EventActorBeginOverlap
  (params (OtherActor :type Actor%20Object%20Reference)))

(event EventTick
  (params (DeltaSeconds :type Float%20%28single-precision%29))
  (if (Variables|Default|GetEventUsed)
    (bind _returnvalue (Actor|GetActorOfClass "/Game/Blueprints/SpookyGhost.SpookyGhost_C"))
    (if (not (Variables|/Game/Blueprints/SpookyGhost.SpookyGhost_C|GetPlayingSpawnAnimation _returnvalue))
      (bind _output_get (Variables|Default|SetGhostDespawnTimer (- (stale _output_get) DeltaSeconds)))
      (if (< _output_get 0.0)
        (bind _returnvalue_2 (Actor|GetActorOfClass "/Game/Blueprints/SpookyGhost.SpookyGhost_C"))
        (Transformation|SetWorldLocation (Variables|/Game/Blueprints/SpookyGhost.SpookyGhost_C|GetGhost _returnvalue_2) "0, 0,-10000.000000" false false)
        (Variables|/Game/Blueprints/SpookyGhost.SpookyGhost_C|SetTrackPlayer _returnvalue_2 false)
        (else
          (CallFunction|InFrame))))))

(fn ConstructionScript)

(fn AddFear
  (params (amnt :type Float%20%28single-precision%29))
  (bind _returnvalue (Actor|GetActorOfClass "/Game/Blueprints/FPSController.FPSController_C"))
  (bind _output_get (Variables|/Game/Blueprints/FPSController.FPSController_C|SetFear _returnvalue (+ (stale _output_get) amnt))))

(fn SetSeverityZero
  (params (ControllerRef :type FPS%20Controller%20Object%20Reference))
  (Variables|Default|SetEventUsed true)
  (Variables|/Game/Blueprints/FPSController.FPSController_C|SetFlashLightEvent ControllerRef true)
  (bind _output_get (Variables|/Game/Blueprints/FPSController.FPSController_C|SetTotalFlickerTime ControllerRef 3.5))
  (Variables|Default|SetGhostDespawnTimer (- _output_get 0.5))
  (Variables|/Game/Blueprints/FPSController.FPSController_C|SetFlashlightOffTime ControllerRef 0.1)
  (Variables|/Game/Blueprints/FPSController.FPSController_C|SetFlashlightOnTime ControllerRef 0.5)
  (Variables|Default|SetGhostSpawnDist 1.8e+03)
  (bind _returnvalue (Actor|GetActorOfClass "/Game/Blueprints/SpookyGhost.SpookyGhost_C"))
  (Variables|/Game/Blueprints/SpookyGhost.SpookyGhost_C|SetGhostSpeed _returnvalue 0.0)
  (Default|PlaySpawninMatAnimation _returnvalue)
  (return _returnvalue))

(fn SetSeverityOne
  (params (PlayerControl :type FPS%20Controller%20Object%20Reference))
  (Variables|Default|SetEventUsed true)
  (Variables|/Game/Blueprints/FPSController.FPSController_C|SetFlashLightEvent PlayerControl true)
  (bind _output_get (Variables|/Game/Blueprints/FPSController.FPSController_C|SetTotalFlickerTime PlayerControl 2.0))
  (Variables|Default|SetGhostDespawnTimer (- _output_get 0.5))
  (Variables|/Game/Blueprints/FPSController.FPSController_C|SetFlashlightOffTime PlayerControl 0.1)
  (Variables|/Game/Blueprints/FPSController.FPSController_C|SetFlashlightOnTime PlayerControl 0.35)
  (Variables|Default|SetGhostSpawnDist 2e+03)
  (bind _returnvalue (Actor|GetActorOfClass "/Game/Blueprints/SpookyGhost.SpookyGhost_C"))
  (Variables|/Game/Blueprints/SpookyGhost.SpookyGhost_C|SetGhostSpeed _returnvalue 4.5e+02)
  (Default|PlaySpawninMatAnimation _returnvalue)
  (return _returnvalue))

(fn SetGhostLocation
  (params (GhostRef :type Spooky%20Ghost%20Object%20Reference%20%28by%20ref%29) (controller%20ref :type FPS%20Controller%20Object%20Reference))
  (bind _camera (Variables|/Game/Blueprints/FPSController.FPSController_C|GetCamera controller%20ref))
  (bind _returnvalue (Math|Vector|GetForwardVector _camera))
  (Transformation|SetActorLocation GhostRef (+ (* (Math|Vector|MakeVector (.x _returnvalue) (.y _returnvalue) 0.0) (Variables|Default|GetGhostSpawnDist)) (.location (Transformation|GetWorldTransform (Variables|/Script/Engine.Character|GetMesh controller%20ref)))) false false)
  (return GhostRef))

(fn SetSeverityTwo
  (params (PlayerControl :type FPS%20Controller%20Object%20Reference))
  (Variables|Default|SetEventUsed true)
  (Variables|/Game/Blueprints/FPSController.FPSController_C|SetFlashLightEvent PlayerControl true)
  (bind _output_get (Variables|/Game/Blueprints/FPSController.FPSController_C|SetTotalFlickerTime PlayerControl 3.0))
  (Variables|Default|SetGhostDespawnTimer (- _output_get 0.5))
  (Variables|/Game/Blueprints/FPSController.FPSController_C|SetFlashlightOffTime PlayerControl 0.1)
  (Variables|/Game/Blueprints/FPSController.FPSController_C|SetFlashlightOnTime PlayerControl 0.25)
  (Variables|Default|SetGhostSpawnDist 2e+03)
  (bind _returnvalue (Actor|GetActorOfClass "/Game/Blueprints/SpookyGhost.SpookyGhost_C"))
  (Variables|/Game/Blueprints/SpookyGhost.SpookyGhost_C|SetGhostSpeed _returnvalue 5e+02)
  (Default|PlaySpawninMatAnimation _returnvalue)
  (return _returnvalue))

(fn SetSeverityThree
  (params (PlayerControl :type FPS%20Controller%20Object%20Reference))
  (Variables|Default|SetEventUsed true)
  (Variables|/Game/Blueprints/FPSController.FPSController_C|SetFlashLightEvent PlayerControl true)
  (bind _output_get (Variables|/Game/Blueprints/FPSController.FPSController_C|SetTotalFlickerTime PlayerControl 1.75))
  (Variables|Default|SetGhostDespawnTimer (- _output_get 0.5))
  (Variables|/Game/Blueprints/FPSController.FPSController_C|SetFlashlightOffTime PlayerControl 0.1)
  (Variables|/Game/Blueprints/FPSController.FPSController_C|SetFlashlightOnTime PlayerControl 0.2)
  (Variables|Default|SetGhostSpawnDist 2e+03)
  (bind _returnvalue (Actor|GetActorOfClass "/Game/Blueprints/SpookyGhost.SpookyGhost_C"))
  (Variables|/Game/Blueprints/SpookyGhost.SpookyGhost_C|SetGhostSpeed _returnvalue 1e+03)
  (Default|PlaySpawninMatAnimation _returnvalue)
  (return _returnvalue))

(fn InFrame
  (bind _returnvalue (Actor|GetActorOfClass "/Game/Blueprints/FPSController.FPSController_C"))
  (bind _returnvalue_2 (Actor|GetActorOfClass "/Game/Blueprints/SpookyGhost.SpookyGhost_C"))
  (bind _output_get (Variables|Default|SetVecToObject (Math|Vector|Normalize (- (Transformation|GetWorldLocation (Variables|/Game/Blueprints/SpookyGhost.SpookyGhost_C|GetGhost _returnvalue_2)) (Transformation|GetWorldLocation (Variables|/Script/Engine.Character|GetMesh _returnvalue))))))
  (if (> (Math|Vector|DotProduct _output_get (Math|Vector|GetForwardVector (Variables|/Game/Blueprints/FPSController.FPSController_C|GetCamera _returnvalue))) 0.5)
    (CallFunction|AddFear (Variables|Default|GetFearAmount))))