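; SpookyGhost2 is a ghost actor that, while TrackPlayer is enabled, chases the player's FPSController actor.
; BeginPlay multiplies the Ghost component's scale by ScaleFactor.
; Each tracking tick looks up FPSController again, turns Ghost on yaw only with a mesh-axis offset, and moves it straight toward the player's mesh at GhostSpeed.
; Movement is frame-rate independent and unswept, so geometry does not block it.
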(event EventBeginPlay
  (bind _ghost (Variables|Default|GetGhost))
  (Transformation|SetWorldScale3D _ghost (* (Transformation|GetWorldScale _ghost) (Variables|Default|GetScaleFactor))))

(event EventTick
  (params (DeltaSeconds :type Float%20%28single-precision%29))
  (bind _ghost (Variables|Default|GetGhost))
  (if (Variables|Default|GetTrackPlayer)
    (bind _returnvalue (Actor|GetActorOfClass "/Game/Blueprints/FPSController.FPSController_C"))
    (CallFunction|AimTowardsPlayer (Variables|/Script/Engine.Character|GetMesh _returnvalue))
    (Transformation|SetWorldLocation _ghost (+ (Transformation|GetWorldLocation _ghost) (* (Math|Vector|Normalize (- (Transformation|GetWorldLocation (Variables|/Script/Engine.Character|GetMesh _returnvalue)) (Transformation|GetWorldLocation (Variables|Default|GetGhost)))) (* DeltaSeconds (Variables|Default|GetGhostSpeed)))) false false)))

(fn ConstructionScript)

(fn AimTowardsPlayer
  (params (Player :type Skeletal%20Mesh%20Component%20Object%20Reference))
  (bind _ghost (Variables|Default|GetGhost))
  (Transformation|SetWorldRotation _ghost (Math|Rotator|MakeRotator 0.0 0.0 (+ (.yaw (Math|Rotator|FindLookatRotation (Transformation|GetWorldLocation _ghost) (Transformation|GetWorldLocation Player))) -9e+01)) false false))