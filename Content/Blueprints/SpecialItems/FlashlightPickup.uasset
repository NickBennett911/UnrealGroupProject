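; Flashlight pickup actor that highlights with a Niagara effect when looked at and gives the player a flashlight.
; Each Tick it line traces from the FPSController camera for a component tagged FlashlightPickup and tracks whether the player is looking at it.
; The look state toggles the particle system, with a DoOnce gating switch-off when the gaze leaves.
; AttemptPickUp reveals the player's Flashlight component and destroys the pickup, only while looked at.
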(event EventBeginPlay
  (bind _returnvalue (AddComponent|AddNiagaraComponent false))
  (Variables|Default|SetParticalSystem _returnvalue)
  (Components|Activation|ToggleActive _returnvalue)
  (bind _returnvalue_2 (Actor|GetActorOfClass "/Game/Blueprints/FPSController.FPSController_C"))
  (Variables|Default|SetPlayerRef _returnvalue_2))

(event EventTick
  (params (DeltaSeconds :type Float%20%28single-precision%29))
  (bind _particalsystem (Variables|Default|GetParticalSystem))
  (bind _particalsystem_2 (Variables|Default|GetParticalSystem))
  (bind _playerref (Variables|Default|GetPlayerRef))
  (bind _returnvalue (Components|Activation|IsActive _particalsystem_2))
  (bind _camera (Variables|/Game/Blueprints/FPSController.FPSController_C|GetCamera _playerref))
  (bind _returnvalue_2 (Transformation|GetWorldLocation _camera))
  (bind (_outhit _returnvalue_3) (Collision|LineTraceByChannel _returnvalue_2 (+ _returnvalue_2 (* (Math|Vector|GetForwardVector _camera) 1000)) "TraceTypeQuery1" false 0 "ForOneFrame" false))
  (if _returnvalue_3
    (if (Components|ComponentHasTag (.HitComponent (Collision|BreakHitResult _outhit)) "FlashlightPickup")
      (Variables|Default|SetIsLookingAtLight true)
      (if (Variables|Default|GetEmittingLookAtAffect)
        (if (not _returnvalue)
          (Variables|Default|SetEmittingLookAtAffect false))
        (else
          (if _returnvalue
            _
            (else
              (Components|Activation|ToggleActive _particalsystem_2)))
          (Variables|Default|SetEmittingLookAtAffect true)
          (goto _label_2 Reset)))
      (else
        (Variables|Default|SetIsLookingAtLight false :!label _label)
        (Utilities|FlowControl|DoOnce false :!label _label_2
          (:Completed
            (Variables|Default|SetEmittingLookAtAffect false)
            (if (Components|Activation|IsActive _particalsystem)
              (Components|Activation|ToggleActive _particalsystem))))))
    (else
      (goto _label))))

(fn ConstructionScript)

(fn AttemptPickUp
  (if (Variables|Default|GetIsLookingAtLight)
    (Rendering|SetVisibility (Variables|/Game/Blueprints/FPSController.FPSController_C|GetFlashlight (Variables|Default|GetPlayerRef)) true true)
    (Actor|DestroyActor)))