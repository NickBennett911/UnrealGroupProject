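; Parent Blueprint for a trigger-activated prop that flings itself toward the player and raises their fear, once.
; Any overlap with the Box enables physics on the StaticMesh and pushes it toward the FPSController's mesh, using FlingArc as the vertical component and scaling by FlingForce.
; The same overlap adds to the controller's Fear, and HasFlung blocks repeat triggers.
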(event OnComponentBeginOverlap(Box)
  (params (OverlappedComponent :type Primitive%20Component%20Object%20Reference) (OtherActor :type Actor%20Object%20Reference) (OtherComp :type Primitive%20Component%20Object%20Reference) (OtherBodyIndex :type Integer) (bFromSweep :type Boolean) (SweepResult :type Hit%20Result%20Structure%20%28by%20ref%29))
  (bind _returnvalue (Actor|GetActorOfClass "/Game/Blueprints/FPSController.FPSController_C"))
  (if (not (Variables|Default|GetHasFlung))
    (CallFunction|Fling (Variables|/Script/Engine.Character|GetMesh _returnvalue))
    (CallFunction|AddFear 5.0)))

(event EventBeginPlay)

(event Collision|EventActorBeginOverlap
  (params (OtherActor :type Actor%20Object%20Reference)))

(event EventTick
  (params (DeltaSeconds :type Float%20%28single-precision%29)))

(fn ConstructionScript)

(fn Fling
  (params (PlayerSkeletalMesh :type Skeletal%20Mesh%20Component%20Object%20Reference))
  (bind _output_get (Variables|Default|SetVectorToPlaer (- (.location (Transformation|GetWorldTransform PlayerSkeletalMesh)) (.location (Transformation|GetWorldTransform (Variables|Default|GetStaticMesh))))))
  (Physics|SetSimulatePhysics (Variables|Default|GetStaticMesh) true)
  (Physics|AddForce (Variables|Default|GetStaticMesh) (* (Math|Vector|MakeVector (.x _output_get) (.y _output_get) (Variables|Default|GetFlingArc)) (Variables|Default|GetFlingForce)) "None" true)
  (Variables|Default|SethasFlung true)
  (Development|PrintString "Fling"))

(fn AddFear
  (params (ammt :type Float%20%28single-precision%29))
  (bind _returnvalue (Actor|GetActorOfClass "/Game/Blueprints/FPSController.FPSController_C"))
  (bind _output_get (Variables|/Game/Blueprints/FPSController.FPSController_C|SetFear _returnvalue (+ (stale _output_get) ammt))))