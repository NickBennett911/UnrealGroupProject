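; Base actor for a one-shot scare prop that slides by itself when the FPSController player is nearby and looking toward it.
; Tick arms the slide once the player is within SlideRadius and a dot product of camera forward against the mesh-to-Item direction exceeds a threshold.
; The actor then moves along local X without sweep until SlideTimer expires, adding player Fear every frame, unscaled by delta time.
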(event EventBeginPlay)

(event Collision|EventActorBeginOverlap
  (params (OtherActor :type Actor%20Object%20Reference)))

(event EventTick
  (params (DeltaSeconds :type Float%20%28single-precision%29))
  (if (not (Variables|Default|GetisSliding))
    (if (not (Variables|Default|GethasSlid))
      (bind _returnvalue (Actor|GetActorOfClass "/Game/Blueprints/FPSController.FPSController_C"))
      (if (< (Transformation|GetDistanceTo _returnvalue) (Variables|Default|GetSlideRadius))
        (bind _returnvalue_2 (Actor|GetActorOfClass "/Game/Blueprints/FPSController.FPSController_C"))
        (bind _output_get (Variables|Default|SetVectorToObject (Math|Vector|Normalize (- (Transformation|GetWorldLocation (Variables|Default|GetItem)) (Transformation|GetWorldLocation (Variables|/Script/Engine.Character|GetMesh _returnvalue_2))))))
        (if (> (Math|Vector|DotProduct _output_get (Math|Vector|GetForwardVector (Variables|/Game/Blueprints/FPSController.FPSController_C|GetCamera _returnvalue_2))) 0.75)
          (Variables|Default|SetisSliding true))))
    (else
      (Transformation|AddActorLocalOffset (Math|Vector|MakeVector (* DeltaSeconds (Variables|Default|GetSlideSpeed)) 0.0 0.0) false false)
      (CallFunction|AddFear 3.0)
      (bind _output_get_2 (Variables|Default|SetSlideTimer (- (stale _output_get_2) DeltaSeconds)))
      (if (<= (Variables|Default|GetSlideTimer) 0.0)
        (Variables|Default|SetisSliding false)
        (Variables|Default|SethasSlid true)))))

(fn ConstructionScript)

(fn AddFear
  (params (amnt :type Float%20%28single-precision%29))
  (bind _returnvalue (Actor|GetActorOfClass "/Game/Blueprints/FPSController.FPSController_C"))
  (bind _output_get (Variables|/Game/Blueprints/FPSController.FPSController_C|SetFear _returnvalue (+ (stale _output_get) amnt))))