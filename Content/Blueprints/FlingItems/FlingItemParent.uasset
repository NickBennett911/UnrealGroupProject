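; Parent actor for fling items: a static mesh that launches itself toward the player once they come within its fling radius.
; Tick checks distance to the FPSController actor until the first fling, which sets HasFlung so it fires only once.
; Fling enables physics and adds a mass-independent force built from the unnormalized horizontal offset to the player's mesh plus a fixed upward component, then prints a debug string.
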(event EventBeginPlay)

(event Collision|EventActorBeginOverlap
  (params (OtherActor :type Actor%20Object%20Reference)))

(event EventTick
  (params (DeltaSeconds :type Float%20%28single-precision%29))
  (if (not (Variables|Default|GethasFlung))
    (bind _returnvalue (Actor|GetActorOfClass "/Game/Blueprints/FPSController.FPSController_C"))
    (if (< (Transformation|GetDistanceTo _returnvalue) (Variables|Default|GetFlingRadius))
      (CallFunction|Fling (Variables|/Script/Engine.Character|GetMesh _returnvalue)))))

(fn ConstructionScript)

(fn Fling
  (params (PlayerSkeletalMesh :type Skeletal%20Mesh%20Component%20Object%20Reference))
  (bind _output_get (Variables|Default|SetVectorToPlaer (- (.location (Transformation|GetWorldTransform PlayerSkeletalMesh)) (.location (Transformation|GetWorldTransform (Variables|Default|GetStaticMesh))))))
  (Physics|SetSimulatePhysics (Variables|Default|GetStaticMesh) true)
  (Physics|AddForce (Variables|Default|GetStaticMesh) (* (Math|Vector|MakeVector (.x _output_get) (.y _output_get) 3e+02) 100) "None" true)
  (Variables|Default|SethasFlung true)
  (Development|PrintString "Fling"))