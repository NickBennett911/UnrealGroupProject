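; Ghost actor that chases the player while TrackPlayer is enabled, with its Ghost component scaled by ScaleFactor on BeginPlay.
; Each Tick turns the Ghost toward the FPSController's mesh on yaw only, with a 90-degree offset.
; It moves the actor at GhostSpeed without sweep, feeding the Ghost's negated right vector into a local offset.
; GhostSpawnSound restarts whenever it stops during tracking.
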(event EventBeginPlay
  (bind _ghost (Variables|Default|GetGhost))
  (Transformation|SetWorldScale3D _ghost (* (Transformation|GetWorldScale _ghost) (Variables|Default|GetScaleFactor))))

(event Collision|EventActorBeginOverlap
  (params (OtherActor :type Actor%20Object%20Reference)))

(event EventTick
  (params (DeltaSeconds :type Float%20%28single-precision%29))
  (bind _ghostspawnsound (Variables|Default|GetGhostSpawnSound))
  (bind _ghost (Variables|Default|GetGhost))
  (if (Variables|Default|GetTrackPlayer)
    (bind _returnvalue (Actor|GetActorOfClass "/Game/Blueprints/FPSController.FPSController_C"))
    (Transformation|SetWorldRotation _ghost (Math|Rotator|MakeRotator 0.0 0.0 (- (.yaw (Math|Rotator|FindLookatRotation (Transformation|GetWorldLocation (Variables|Default|GetGhost)) (Transformation|GetWorldLocation (Variables|/Script/Engine.Character|GetMesh _returnvalue)))) 9e+01)) false false)
    (Transformation|AddActorLocalOffset (* (* (Math|Vector|GetRightVector _ghost) -1) (* DeltaSeconds (Variables|Default|GetGhostSpeed))) false false)
    (if (not (Audio|Components|Audio|IsPlaying _ghostspawnsound))
      (Audio|Components|Audio|Play _ghostspawnsound 0.0))))

(fn ConstructionScript)