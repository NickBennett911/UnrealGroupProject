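; First-person player character with mouse look, yaw-relative movement, jumping and a flashlight that follows the camera.
; Input events feed controller yaw, pitch and movement directly.
; Every Tick places the flashlight ahead of the camera with a swept move, applies a local offset, then aligns it to the camera's forward vector.
; Disconnected nodes hold an alternative placement and a flashlight-to-camera distance tolerance check that never run.
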(event EventTick
  (params (DeltaSeconds :type Float%20%28single-precision%29))
  (bind _camera (Variables|Default|GetCamera))
  (Transformation|SetWorldLocation (Variables|Default|GetFlashlight) (+ (* (Math|Vector|GetForwardVector _camera) 3e+01) (Transformation|GetWorldLocation _camera)) true false)
  (Transformation|AddLocalOffset (Variables|Default|GetFlashlight) "0,20.000000,-20.000000" false false)
  (Transformation|SetWorldRotation (Variables|Default|GetFlashlight) (Math|Rotator|MakeRotationfromAxes (Math|Vector|GetForwardVector (Variables|Default|GetCamera)) "0, 0, 0" "0, 0, 0") false false))

(event Input|ActionEvents|InputActionJump
  (params (Key :type Key%20Structure :default "None"))
  (:Pressed
    (Character|Jump)))

(event Input|AxisEvents|InputAxisMouseLookHorizontal
  (params (AxisValue :type Float%20%28single-precision%29))
  ;[1 1 1] Character Look
  (Pawn|Input|AddControllerYawInput AxisValue))

(event Input|AxisEvents|InputAxisMouseLookVertical
  (params (AxisValue :type Float%20%28single-precision%29))
  ;[1 1 1] Character Look
  (Pawn|Input|AddControllerPitchInput AxisValue))

(event Input|AxisEvents|InputAxisHorizontal
  (params (AxisValue :type Float%20%28single-precision%29))
  (Pawn|Input|AddMovementInput (Math|Vector|GetRightVector (Math|Rotator|MakeRotator 0.0 0.0 (.yaw (Pawn|GetControlRotation :!class /Script/Engine.Pawn)))) AxisValue false))

(event Input|AxisEvents|InputAxisVertical
  (params (AxisValue :type Float%20%28single-precision%29))
  (Pawn|Input|AddMovementInput (Math|Vector|GetForwardVector (Math|Rotator|MakeRotator 0.0 0.0 (.yaw (Pawn|GetControlRotation :!class /Script/Engine.Pawn)))) AxisValue false))

(fn ConstructionScript)

(fn GetFlashlighttoCameraDistance
  (return (Math|Vector|VectorLength (- (Transformation|GetWorldLocation (Variables|Default|GetCamera)) (Transformation|GetWorldLocation (Variables|Default|GetFlashlight))))))