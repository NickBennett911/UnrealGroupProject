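; Ghost event manager that scatters flashlight flicker, spawn-behind-player and sound scares across hard-coded map locations at BeginPlay.
; SpawnSpecificGhostEvents spawns set counts of each type, scaling flicker and spawn-behind severity by the FPSController's visited-place count.
; GetEventLocation draws random spots without repeats from a temporary list, destroying any GhostEvent-tagged actor already there.
; SpawnGhostEvents offers random-type spawning but is not called here, and resets the list after every spawn.
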(event OnComponentBeginOverlap(TestCollider)
  (params (OverlappedComponent :type Primitive%20Component%20Object%20Reference) (OtherActor :type Actor%20Object%20Reference) (OtherComp :type Primitive%20Component%20Object%20Reference) (OtherBodyIndex :type Integer) (bFromSweep :type Boolean) (SweepResult :type Hit%20Result%20Structure%20%28by%20ref%29)))

(event EventBeginPlay
  (CallFunction|MakeList)
  (CallFunction|SpawnSpecificGhostEvents 1 2 3))

(event Collision|EventActorBeginOverlap
  (params (OtherActor :type Actor%20Object%20Reference)))

(event EventTick
  (params (DeltaSeconds :type Float%20%28single-precision%29)))

(fn ConstructionScript)

(fn MakeList
  (bind _output_get (Variables|Default|SetMasterLocations (Utilities|Array|MakeArray (Math|Vector|MakeVector 289.0 -2086.0 58.0) (Math|Vector|MakeVector 1332.0 -1349.0 136.0) (Math|Vector|MakeVector 363.0 -993.0 105.0) (Math|Vector|MakeVector -751.0 839.0 58.0) (Math|Vector|MakeVector -1908.0 -605.0 58.0) (Math|Vector|MakeVector -2189.0 524.0 58.0) (Math|Vector|MakeVector -928.0 1364.0 58.0) (Math|Vector|MakeVector 223.0 459.0 94.0) (Math|Vector|MakeVector 2149.0 -1564.0 58.0) (Math|Vector|MakeVector 2433.0 3.4e+02 58.0) (Math|Vector|MakeVector 2436.0 1948.0 58.0) (Math|Vector|MakeVector 2.88e+03 3401.0 58.0) (Math|Vector|MakeVector 7.9e+02 2394.0 136.0) (Math|Vector|MakeVector -96.0 4561.0 58.0) (Math|Vector|MakeVector 2276.0 4395.0 6e+02) (Math|Vector|MakeVector 1.17e+03 3669.0 144.0) (Math|Vector|MakeVector -714.0 1991.0 77.0))))
  (Variables|Default|SetTempLocations _output_get))

(fn SpawnGhostEvents
  (params (NumEvents :type Integer))
  (bind _result (Math|Integer|DecrementInt NumEvents)
    (:%20%20
      (for _index (range 0 _result)
        (bind _location (CallFunction|GetEventLocation))
        (LocalVariables|SetEventLocation _location)
        (switch int (Math|Random|RandomIntegerinRange 0 (- (Variables|Default|GetNumOfGhostEvents) 1))
          (:0
            (bind _returnvalue (Game|SpawnActorfromClass "/Game/Blueprints/GhostEvents/SpawnBehindPlayerEvent.SpawnBehindPlayerEvent_C" (LocalVariables|GetEventLocation) "Undefined" 0 0))
            (Default|SetEventSeverity _returnvalue (Variables|Default|GetCurNumVisitedPlaces)))
          (:1
            (Game|SpawnActorfromClass "/Game/Blueprints/GhostEvents/SoundEventParent.SoundEventParent_C" (LocalVariables|GetEventLocation) "Undefined" 0 0))
          (:2
            (bind _returnvalue_2 (Game|SpawnActorfromClass "/Game/Blueprints/GhostEvents/FlashlightFlickerEvent.FlashlightFlickerEvent_C" (LocalVariables|GetEventLocation) "Undefined" 0 0))
            (Variables|/Game/Blueprints/GhostEvents/FlashlightFlickerEvent.FlashlightFlickerEvent_C|SetSeverityLevel _returnvalue_2 (Variables|Default|GetCurNumVisitedPlaces))))
        (Variables|Default|SetTempLocations (Variables|Default|GetMasterLocations))))))

(fn GetEventLocation
  (bind _templocations (Variables|Default|GetTempLocations))
  (LocalVariables|SetIndexChosen (Math|Random|RandomIntegerinRange 0 (- (Utilities|Array|Length _templocations) 1)))
  (CallFunction|ClearChoosenSpot (Utilities|Array|Get(acopy) _templocations (LocalVariables|GetIndexChosen)))
  (LocalVariables|SetCurLocation (Math|Transform|MakeTransform (Utilities|Array|Get(acopy) _templocations (LocalVariables|GetIndexChosen))))
  (Utilities|Array|RemoveIndex (Variables|Default|GetTempLocations) (LocalVariables|GetIndexChosen))
  (return (LocalVariables|GetCurLocation)))

(fn SpawnSpecificGhostEvents
  (params (Flashlight :type Integer) (SpawnBehind :type Integer) (Sound :type Integer))
  (bind _returnvalue (Actor|GetActorOfClass "/Game/Blueprints/FPSController.FPSController_C"))
  (Variables|Default|SetCurNumVisitedPlaces (Variables|/Game/Blueprints/FPSController.FPSController_C|GetPlacesVisited _returnvalue))
  (bind _result (Math|Integer|DecrementInt Flashlight)
    (:%20%20
      (for _index (range 0 _result)
        (bind _location (CallFunction|GetEventLocation))
        (bind _returnvalue_2 (Game|SpawnActorfromClass "/Game/Blueprints/GhostEvents/FlashlightFlickerEvent.FlashlightFlickerEvent_C" _location "Undefined" 0 0))
        (Variables|/Game/Blueprints/GhostEvents/FlashlightFlickerEvent.FlashlightFlickerEvent_C|SetSeverityLevel _returnvalue_2 (Variables|Default|GetCurNumVisitedPlaces)))
      (bind _result_2 (Math|Integer|DecrementInt SpawnBehind)
        (:%20%20
          (for _index_2 (range 0 _result_2)
            (bind _location_2 (CallFunction|GetEventLocation))
            (bind _returnvalue_3 (Game|SpawnActorfromClass "/Game/Blueprints/GhostEvents/SpawnBehindPlayerEvent.SpawnBehindPlayerEvent_C" _location_2 "Undefined" 0 0))
            (Default|SetEventSeverity _returnvalue_3 (Variables|Default|GetCurNumVisitedPlaces)))
          (bind _result_3 (Math|Integer|DecrementInt Sound)
            (:%20%20
              (for _index_3 (range 0 _result_3)
                (bind _location_3 (CallFunction|GetEventLocation))
                (Game|SpawnActorfromClass "/Game/Blueprints/GhostEvents/SoundEventParent.SoundEventParent_C" _location_3 "Undefined" 0 0))
              (Variables|Default|SetTempLocations (Variables|Default|GetMasterLocations)))))))))

(fn ClearChoosenSpot
  (params (Location :type Vector%20%28by%20ref%29))
  (bind _outactors (Actor|GetAllActorswithTag "GhostEvent"))
  (bind _array_element (Utilities|Array|ForEachLoopwithBreak _outactors :!label _label)
    (:LoopBody
      (if (Math|Vector|Equal(Vector) (Transformation|GetActorLocation _array_element) Location 1e+01)
        (Actor|DestroyActor _array_element)
        (goto _label Break)))))