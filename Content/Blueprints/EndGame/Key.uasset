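; Key actor for the end game, built around a Cube component whose visibility is meant to follow the FPSController's CanDie flag.
; It hides the Cube on BeginPlay, then looks up the FPSController every Tick and calls Show while CanDie is true.
; Show sets visibility to false just as Hide does, so the Cube stays hidden as written.
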(event EventBeginPlay
  (CallFunction|Hide))

(event Collision|EventActorBeginOverlap
  (params (OtherActor :type Actor%20Object%20Reference)))

(event EventTick
  (params (DeltaSeconds :type Float%20%28single-precision%29))
  (bind _returnvalue (Actor|GetActorOfClass "/Game/Blueprints/FPSController.FPSController_C"))
  (if (Variables|/Game/Blueprints/FPSController.FPSController_C|GetCanDie _returnvalue)
    (CallFunction|Show)))

(fn ConstructionScript)

(fn Hide
  (Rendering|SetVisibility (Variables|Default|GetCube) false false))

(fn Show
  (Rendering|SetVisibility (Variables|Default|GetCube) false false))